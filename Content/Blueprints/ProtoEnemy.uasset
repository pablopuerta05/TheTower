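; Prototype enemy character that knocks the player away when it hits them.
; On a hit with a Player-tagged first-person character, it launches that character along its own forward vector scaled by Force, overriding existing velocity.
; BeginPlay calls SetBotMovementSpeed to zero both walk and crouch speeds, so the enemy stands still.
; AI chase and self-spawn logic are present but unconnected, and Tick is empty.
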(event `self.ReceiveHit`
  (params (MyComp :type "PrimitiveComponent Object Reference") (Other :type "Actor Object Reference") (OtherComp :type "PrimitiveComponent Object Reference") (bSelfMoved :type Boolean) (HitLocation :type "Vector Structure") (HitNormal :type "Vector Structure") (NormalImpulse :type "Vector Structure") (Hit :type "HitResult Structure (by ref)"))
  ; Launch player on collision
  (if (`self.ActorHasTag` Other "Player")
    (bind _asbp_first_person_character (cast `/Game/FirstPerson/Blueprints/BP_FirstPersonCharacter` Other))
    (`self.LaunchCharacter` _asbp_first_person_character (* (`self.GetActorForwardVector` self) (`self.Force`)) true true)))

(event `self.ReceiveTick`
  (params (DeltaSeconds :type "Float (single-precision)"))
  ; AI move to player
)

(event `self.ReceiveBeginPlay`
  ; Begin play
  (`self.SetBotMovementSpeed` 0.0))

(fn `SetBotMovementSpeed`
  (params (MoveSpeed :type "Float (double-precision)"))
  (bind _charactermovement (`self.CharacterMovement`))
  (set `CharacterMovementComponent.MaxWalkSpeed` MoveSpeed _charactermovement)
  (set `CharacterMovementComponent.MaxWalkSpeedCrouched` MoveSpeed _charactermovement))

(fn `UserConstructionScript`)