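; Movable platform actor that slides along the world X axis between two positions.
; BeginPlay starts the Movement timeline, whose updates switch on Type to pick the motion.
; Type 0, the only implemented case, calls MovX to lerp X between Posicion1 and Posicion2, keeping Y and Z, without sweep.
; Any other Type prints an error and resets to 0.
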(event `self.ReceiveBeginPlay`
  (bind (_direction _position) (`Timeline|Movement` :`NewTime` (`GameplayStatics.GetWorldDeltaSeconds`))
    (:`Update`
      (switch `int` (`self.Type`)
        (:`Default`
          (`KismetSystemLibrary.PrintString` "Error")
          (set `self.Type` 0))
        (:`0`
          (`self.MovX` _position (`self.Posicion1`) (`self.Posicion2`)))))))

(event `self.ReceiveTick`
  (params (DeltaSeconds :type "Float (single-precision)")))

(fn `MovX`
  (params (AlphaProgress :type "Float (double-precision)") (a :type "Float (double-precision)") (b :type "Float (double-precision)"))
  (bind (_returnvalue_x _returnvalue_y _returnvalue_z) (`KismetMathLibrary.BreakVector` (`self.K2_GetActorLocation`)))
  (`self.K2_SetActorLocation` (`KismetMathLibrary.MakeVector` (`KismetMathLibrary.Lerp` a b AlphaProgress) _returnvalue_y _returnvalue_z)))

(fn `UserConstructionScript`)